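; Archer gameplay ability that lets the enemy archer shove characters with its bow.
; The Push function binds PushEnemy to the BowCollision begin-overlap on BP_EnemyArcher, and ending the ability unbinds it.
; PushEnemy launches any overlapping GASProjectCharacter other than the avatar, scaling PushStrength by the Roll and Pitch of the avatar's eye-view rotation for X and Y velocity, rather than a direction vector.
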(event Custom|PushEnemy
  (params (OverlappedComponent :type Primitive%20Component%20Object%20Reference) (OtherActor :type Actor%20Object%20Reference) (OtherComp :type Primitive%20Component%20Object%20Reference) (OtherBodyIndex :type Integer) (bFromSweep :type Boolean) (SweepResult :type Hit%20Result%20Structure%20%28by%20ref%29))
  (bind _returnvalue (Ability|GetAvatarActorfromActorInfo))
  (bind _pushstrength (Variables|Default|GetPushStrength))
  (bind _outrotation (Actor|GetActorEyesViewPoint _returnvalue))
  (if (!= OtherActor (Ability|GetAvatarActorfromActorInfo))
    (bind _asgasproject_character (Utilities|Casting|CastToGASProjectCharacter OtherActor))
    (Character|LaunchCharacter _asgasproject_character (Math|Vector|MakeVector (* _pushstrength (.roll _outrotation)) (* _pushstrength (.pitch _outrotation)) 0.0) false false)))

(event Ability|EventOnEndAbility
  (params (bWasCancelled :type Boolean))
  (|CallParentFunction bWasCancelled)
  (bind _asbp_enemy_archer (Utilities|Casting|CastToBP_EnemyArcher (Ability|GetAvatarActorfromActorInfo)))
  (Collision|UnbindEventfromOnComponentBeginOverlap (Variables|/Game/ThirdPerson/Blueprints/BP_EnemyArcher.BP_EnemyArcher_C|GetBowCollision _asbp_enemy_archer) (delegate Custom|PushEnemy)))

(fn Push
  (bind _asbp_enemy_archer (Utilities|Casting|CastToBP_EnemyArcher (Ability|GetAvatarActorfromActorInfo)))
  (Collision|BindEventtoOnComponentBeginOverlap (Variables|/Game/ThirdPerson/Blueprints/BP_EnemyArcher.BP_EnemyArcher_C|GetBowCollision _asbp_enemy_archer) (EventDispatchers|CreateEvent :!event Custom|PushEnemy)))