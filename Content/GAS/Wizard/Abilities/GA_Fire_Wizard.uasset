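; Wizard fire gameplay ability that supplies the projectile spawn step, launching a BP_MagicBullet with random spread.
; SpawnProjectile builds the bullet's rotation by nudging the forward axis with small random offsets along the right and up axes, then passes the owner and effect spec handle to the spawned actor.
; Activation and end events are disabled placeholders, so that logic is left to the parent class.
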(event Ability|EventActivateAbility
  (|CallParentFunction) ; This node is disabled and will not be called.\nDrag off pins to build functionality.
)

(event Ability|EventOnEndAbility
  (params (bWasCancelled :type Boolean))
  (|CallParentFunction bWasCancelled) ; This node is disabled and will not be called.\nDrag off pins to build functionality.
)

(fn SpawnProjectile
  (params (SpawnTransformLocation :type Vector :default "0, 0, 0") (SpawnTransformRotation :type Rotator :default "0, 0, 0") (Owner :type Actor%20Object%20Reference) (SpecHandle :type Gameplay%20Effect%20Spec%20Handle%20Structure))
  (bind (_x _y _z) (Math|Rotator|GetAxes SpawnTransformRotation))
  (Game|SpawnActorfromClass "/Game/ThirdPerson/Blueprints/Projectiles/BP_MagicBullet.BP_MagicBullet_C" (Math|Transform|MakeTransform SpawnTransformLocation (Math|Rotator|MakeRotfromX (+ (+ _x (* _z (Math|Random|RandomFloatinRange -0.1 0.1))) (* _y (Math|Random|RandomFloatinRange -0.1 0.1)))) "1.000000,1.000000,1.000000") "Undefined" "MultiplyWithRoot" Owner SpecHandle 0))