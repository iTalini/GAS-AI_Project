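; Gameplay ability for the AI wizard that fakes a teleport as a very fast, invisible flight to a teleportation point.
; It commits SetByCaller cost and cooldown, hides the wizard, then on a montage notify enables flying, ignores pawn collision, attaches a Niagara trail and runs AIMoveTo.
; Arrival or failure restores defaults and plays the ending montage, with a timer as failsafe.
; Ending clears the timer and trail and fires the wizard's teleport-end delegate.
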(event Custom|FinishAbility
  (CallFunction|SetParameterstoDefault)
  (Ability|EndAbility))

(event Ability|EventActivateAbility
  (CallFunction|AssignTags)
  (bind _returnvalue (Ability|CommitAbility))
  (if _returnvalue
    (Utilities|Casting|CastToGAS_AICharacter_Wizard (Ability|GetAvatarActorfromActorInfo)
      (:then
        (Variables|Default|SetWizardOwner 0)
        (Animation|Montage|MontageStop -1.0)
        (bind _notifyname (Animation|Montage|PlayMontage (Variables|/Script/Engine.Character|GetMesh (Variables|Default|GetWizardOwner)) "/Game/Characters/MIXAMO/Wizard/Animation/AM_Magic_Teleport.AM_Magic_Teleport")
          (:then
            (Default|MakeWizardInvisible (Variables|Default|GetWizardOwner))
            (bind _returnvalue_2 (Utilities|Time|SetTimerbyEvent (delegate Custom|FinishAbility) 5.0))
            (Variables|Default|SetEmergencyOfAbility _returnvalue_2))
          (:OnNotifyBegin
            (switch name _notifyname
              (:Teleport
                (Animation|Montage|MontageStop -1.0)
                (Pawn|Components|CharacterMovement|SetMovementMode (Variables|/Script/Engine.Character|GetCharacterMovement (Variables|Default|GetWizardOwner)) "MOVE_Flying" 0)
                (Variables|/Script/Engine.CharacterMovementComponent|SetMaxFlySpeed (Variables|/Script/Engine.Character|GetCharacterMovement (Variables|Default|GetWizardOwner)) 5e+03)
                (Variables|/Script/Engine.CharacterMovementComponent|SetMaxAcceleration (Variables|/Script/Engine.Character|GetCharacterMovement (Variables|Default|GetWizardOwner)) 99999.0)
                (Collision|SetCollisionResponsetoChannel (Variables|/Script/Engine.Character|GetCapsuleComponent (Variables|Default|GetWizardOwner)) "ECC_Pawn" "ECR_Ignore")
                (bind _returnvalue_3 (Niagara|SpawnSystemAttached "/Game/Niagara/N_TrailsOfDeath.N_TrailsOfDeath" (Variables|/Script/Engine.Character|GetMesh (Variables|Default|GetWizardOwner)) "Hips" "0, 0, 0" "0, 0, 0" "KeepRelativeOffset" false))
                (Variables|Default|SetTeleportBodyEffect _returnvalue_3)
                (bind _wizardowner (Variables|Default|GetWizardOwner)
                  (:then
                    (AI|AIMoveTo _wizardowner (Default|GetTeleportationPoint _wizardowner) 0 15.0 false
                      (:OnSuccess
                        _)
                      (:OnFail
                        _))
                    (CallFunction|SetParameterstoDefault)
                    (Animation|Montage|PlayMontage (Variables|/Script/Engine.Character|GetMesh (Variables|Default|GetWizardOwner)) "/Game/Characters/MIXAMO/Wizard/Animation/AM_Magic_Teleport.AM_Magic_Teleport" 1.0 0.0 "TeleportEnding"
                      (:OnCompleted
                        _)
                      (:OnBlendOut
                        _)
                      (:OnInterrupted
                        _))
                    (Ability|EndAbility))
                  (:else
                    (CallFunction|SetParameterstoDefault)
                    (Ability|EndAbility))))))))
      (:CastFailed
        (Ability|EndAbility :!label _label)))
    (else
      (goto _label))))

(event Ability|EventOnEndAbility
  (params (bWasCancelled :type Boolean))
  (Utilities|Time|ClearandInvalidateTimerbyHandle (Variables|Default|GetEmergencyOfAbility))
  (Utilities|FlowControl|Sequence
    (:then_0
      (bind _wizardowner (Variables|Default|GetWizardOwner)
        (:then
          (Class|GASAICharacterWizard|CallonTeleportEndDelegate _wizardowner))
        (:else)))
    (:then_1
      (bind _teleportbodyeffect (Variables|Default|GetTeleportBodyEffect)
        (:then
          (Components|DestroyComponent _teleportbodyeffect))
        (:else)))))

(fn AssignTags
  (Ability|GameplayEffect|AssignTagSetbyCallerMagnitude (Ability|MakeOutgoingGameplayEffectSpec (Class|GASGABaseAbility|GetAbilityCostClass)) (Variables|Default|GetAbilityCostEffectTag) (.value (Class|GASGABaseAbility|GetCostValue)))
  (Ability|GameplayEffect|AssignTagSetbyCallerMagnitude (Ability|MakeOutgoingGameplayEffectSpec (Class|GASGABaseAbility|GetCooldownClass)) (Variables|Default|GetCooldownEffectTag) (.value (Class|GASGABaseAbility|GetCooldownDuration))))

(fn SetParameterstoDefault
  (bind _wizardowner (Variables|Default|GetWizardOwner))
  (bind _charactermovement (Variables|/Script/Engine.Character|GetCharacterMovement _wizardowner))
  (Pawn|Components|CharacterMovement|SetMovementMode _charactermovement "MOVE_Walking" 0)
  (Variables|/Script/Engine.CharacterMovementComponent|SetMaxAcceleration _charactermovement 1.5e+03)
  (Collision|SetCollisionResponsetoChannel (Variables|/Script/Engine.Character|GetCapsuleComponent (Variables|Default|GetWizardOwner)) "ECC_Pawn" "ECR_Block")
  (Default|MakeWizardVisible (Variables|Default|GetWizardOwner)))