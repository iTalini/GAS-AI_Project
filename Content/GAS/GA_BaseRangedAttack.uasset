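; Base Gameplay Ability for ranged attacks, with SpawnProjectile as the override point for projectile types (BP_Arrow here).
; ActivateAbility and OnEndAbility are empty; the attack and cleanup chains are unwired and never run.
; The unwired attack chains a root-motion dash into an attack montage, whose notifies pause movement and fire from an AI character's right weapon along controller rotation.
; Projectiles carry a SetByCaller damage effect spec.
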(event Ability|EventActivateAbility)

(event Ability|EventOnEndAbility
  (params (bWasCancelled :type Boolean)))

(fn SpawnProjectile
  (params (SpawnTransformLocation :type Vector) (SpawnTransformRotation :type Rotator) (Owner :type Actor%20Object%20Reference) (SpecHandle :type Gameplay%20Effect%20Spec%20Handle%20Structure))
  (Game|SpawnActorfromClass "/Game/ThirdPerson/Blueprints/Projectiles/BP_Arrow.BP_Arrow_C" (Math|Transform|MakeTransform SpawnTransformLocation SpawnTransformRotation "1.000000,1.000000,1.000000") "Undefined" "MultiplyWithRoot" Owner SpecHandle 0)
  (return))