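; Base Gameplay Ability for blocking, shared by player and AI characters.
; Activation builds set-by-caller cost and cooldown specs, commits, adds a Status.Blocking actor tag and plays the block montage, whose Start Block notify applies GE_Block.
; Players stop through WaitCancel and AI through a timer, both playing the montage's End section.
; Ending removes the tag and calls the character's block-ended delegate.
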(event Custom|StopAbility
  (bind _skeletalmesh (Variables|Default|GetSkeletalMesh))
  (Utilities|FlowControl|DoOnce false
    (:Completed
      (Utilities|IsValid _skeletalmesh
        (:Is%20Valid
          (Animation|Montage|MontageStop -1.0)
          (Animation|Montage|PlayMontage _skeletalmesh (Variables|Default|GetBlockAnimation) 1.0 0.0 "End"
            (:OnCompleted
              _)
            (:OnBlendOut
              _)
            (:OnInterrupted
              _))
          (Ability|EndAbility))
        (:Is%20Not%20Valid
          (Ability|EndAbility))))))

(event Ability|EventActivateAbility
  (bind _returnvalue (Ability|GetAvatarActorfromActorInfo))
  (CallFunction|AssignTags)
  (Ability|CommitAbility)
  (bind _asgasproject_character (Utilities|Casting|CastToGASProjectCharacter (Ability|GetAvatarActorfromActorInfo))
    (:then
      (Variables|Default|SetSkeletalMesh (Variables|/Script/Engine.Character|GetMesh _asgasproject_character))
      (Utilities|Array|AddUnique (Variables|/Script/Engine.Actor|GetTags _asgasproject_character) "Status.Blocking")
      (bind _notifyname (Animation|Montage|PlayMontage (Variables|Default|GetSkeletalMesh) (Variables|Default|GetBlockAnimation))
        (:then
          (Utilities|Casting|CastToGAS_AICharacter _returnvalue
            (:then
              (Utilities|Time|SetTimerbyEvent (delegate Custom|StopAbility) 3.0))
            (:CastFailed
              (Utilities|Casting|CastToGAS_PlayerCharacter _returnvalue
                (:then
                  (|WaitCancel
                    (:OnCancel
                      (Utilities|IsValid (Variables|Default|GetSkeletalMesh)
                        (:Is%20Valid
                          (Animation|Montage|MontageStop -1.0)
                          (Animation|Montage|PlayMontage (Variables|Default|GetSkeletalMesh) (Variables|Default|GetBlockAnimation) 1.0 0.0 "End"
                            (:OnCompleted
                              _)
                            (:OnBlendOut
                              _)
                            (:OnInterrupted
                              _))
                          (Ability|EndAbility))
                        (:Is%20Not%20Valid
                          (Ability|EndAbility))))))
                (:CastFailed
                  (Ability|EndAbility))))))
        (:OnCompleted
          (Ability|EndAbility :!label _label))
        (:OnBlendOut
          (goto _label))
        (:OnNotifyBegin
          (switch name _notifyname
            (:StartBlock
              (Utilities|FlowControl|DoOnce false
                (:Completed
                  (Ability|ApplyGameplayEffectToOwner "/Game/GAS/Common/Effects/GE_Block.GE_Block_C"))))))))
    (:CastFailed
      (Ability|EndAbility))))

(event Ability|EventOnEndAbility
  (params (bWasCancelled :type Boolean))
  (bind _asgasproject_character (Utilities|Casting|CastToGASProjectCharacter (Ability|GetAvatarActorfromActorInfo)))
  (Utilities|Array|RemoveItem (Variables|/Script/Engine.Actor|GetTags _asgasproject_character) "Status.Blocking")
  (Class|GASProjectCharacter|CallonBlockEndedDelegate _asgasproject_character))

(fn AssignTags
  (Ability|GameplayEffect|AssignTagSetbyCallerMagnitude (Ability|MakeOutgoingGameplayEffectSpec (Class|GASGABaseAbility|GetAbilityCostClass)) (Variables|Default|GetAbilityCostEffectTag) (.value (Class|GASGABaseAbility|GetCostValue)))
  (Ability|GameplayEffect|AssignTagSetbyCallerMagnitude (Ability|MakeOutgoingGameplayEffectSpec (Class|GASGABaseAbility|GetCooldownClass)) (Variables|Default|GetCooldownEffectTag) (.value (Class|GASGABaseAbility|GetCooldownDuration))))