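; Gameplay Ability that runs passive health regeneration on its owner through the GE_PassiveRegenHealth effect.
; On activation it applies the effect, stores the handle, and starts an async attribute-ratio threshold task.
; The ability ends itself when the watched ratio changes to exactly 1.0, presumably full health.
; Ending removes all stacks of the effect by handle and stops the task.
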(event Ability|EventActivateAbility
  (bind _returnvalue (Ability|ApplyGameplayEffectToOwner "/Game/GAS/Common/Effects/GE_PassiveRegenHealth.GE_PassiveRegenHealth_C"))
  (Variables|Default|SetRegenHealthGE _returnvalue)
  (bind (_asynctaskproxy _bmatchescomparison) (|WaitforAttributeChangeRatioThreshold "(AttributeName=\"Health\",Attribute=/Script/GASProject.GAS_AttributeSet:Health,AttributeOwner=\"/Script/CoreUObject.Class'/Script/GASProject.GAS_AttributeSet'\")" "(AttributeName=\"MaxHealth\",Attribute=/Script/GASProject.GAS_AttributeSet:MaxHealth,AttributeOwner=\"/Script/CoreUObject.Class'/Script/GASProject.GAS_AttributeSet'\")" "ExactlyEqualTo" 1.0 false 0)
    (:then
      (Variables|Default|SetAsync%20Task _asynctaskproxy))
    (:OnChange
      (if _bmatchescomparison
        (Ability|EndAbility)))))

(event Ability|EventOnEndAbility
  (params (bWasCancelled :type Boolean))
  (Ability|RemoveGameplayEffectFromOwnerWithHandle (Variables|Default|GetRegenHealthGE))
  (GameplayTasks|EndTask (Variables|Default|GetAsync%20Task)))