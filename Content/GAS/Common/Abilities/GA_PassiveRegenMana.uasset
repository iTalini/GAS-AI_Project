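; GA_PassiveRegenMana is a Gameplay Ability that regenerates the owner's mana through a gameplay effect.
; On activation it applies GE_PassiveRegenMana, stores the handle and starts an async wait on an attribute ratio.
; The ability ends itself when that ratio changes to exactly 1.0.
; On end it removes the effect by its handle and ends the async task.
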(event Ability|EventActivateAbility
  (bind _returnvalue (Ability|ApplyGameplayEffectToOwner "/Game/GAS/Common/Effects/GE_PassiveRegenMana.GE_PassiveRegenMana_C"))
  (Variables|Default|SetRegenManaGE _returnvalue)
  (bind (_asynctaskproxy _bmatchescomparison) (|WaitforAttributeChangeRatioThreshold "(AttributeName=\"Mana\",Attribute=/Script/GASProject.GAS_AttributeSet:Mana,AttributeOwner=\"/Script/CoreUObject.Class'/Script/GASProject.GAS_AttributeSet'\")" "(AttributeName=\"MaxMana\",Attribute=/Script/GASProject.GAS_AttributeSet:MaxMana,AttributeOwner=\"/Script/CoreUObject.Class'/Script/GASProject.GAS_AttributeSet'\")" "ExactlyEqualTo" 1.0 false 0)
    (:then
      (Variables|Default|SetAsync%20Task _asynctaskproxy))
    (:OnChange
      (if _bmatchescomparison
        (Ability|EndAbility)))))

(event Ability|EventOnEndAbility
  (params (bWasCancelled :type Boolean))
  (Ability|RemoveGameplayEffectFromOwnerWithHandle (Variables|Default|GetRegenManaGE))
  (GameplayTasks|EndTask (Variables|Default|GetAsync%20Task)))